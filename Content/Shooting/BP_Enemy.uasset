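; BP_Enemy is a shooting-game enemy that flies toward the player and destroys itself along with whatever it hits.
; On BeginPlay it finds BP_Player and stores a normalized direction toward that position, computed once, so it does not home.
; Tick moves it along that direction at Speed, scaled by delta time and without sweep.
; A Cube overlap destroys both the other actor and the enemy, with no filtering.
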(event `self.ReceiveBeginPlay`
  ;[1 1 1] Target 이 있어야 한다.
  (bind _returnvalue (`GameplayStatics.GetActorOfClass` "/Game/Shooting/BP_Player.BP_Player_C"))
  (set `self.Target` _returnvalue)
  (set `self.Direction` (`KismetMathLibrary.Normal` (- (`self.K2_GetActorLocation` (`self.Target`)) (`self.K2_GetActorLocation`)))))

(event `self.ReceiveTick`
  (params (DeltaSeconds :type "Float (single-precision)"))
  ;[1 1 1] 이동하고싶다.
  ;;[1 1 1] P
  (`self.K2_SetActorLocation` (+ (* DeltaSeconds (* (`self.Direction`) (`self.Speed`))) (`self.K2_GetActorLocation`))))

(event `self.Cube.OnComponentBeginOverlap`
  (params (OverlappedComponent :type "PrimitiveComponent Object Reference") (OtherActor :type "Actor Object Reference") (OtherComp :type "PrimitiveComponent Object Reference") (OtherBodyIndex :type Integer) (bFromSweep :type Boolean) (SweepResult :type "HitResult Structure (by ref)"))
  (`self.K2_DestroyActor` OtherActor)
  (`self.K2_DestroyActor`))

(fn `UserConstructionScript`)