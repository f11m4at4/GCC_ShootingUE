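; BP_EnemyGOD is an enemy spawner actor for the shooting game that repeatedly spawns BP_Enemy at its own location.
; Tick passes delta time to TimeFlow, which accumulates it in CurrentTime.
; When CurrentTime exceeds CreateTime, it spawns an enemy and resets the counter to zero, giving a fixed-interval spawn loop without timers.
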(event `self.ReceiveTick`
  (params (DeltaSeconds :type "Float (single-precision)"))
  ;[1 1 1] 시간이 흘러야한다.
  (`self.TimeFlow` DeltaSeconds)
  ;[1 1 1] 만약 경과시간이 생성시간을 초과했다면
  (if (> (`self.CurrentTime`) (`self.CreateTime`))
    ;[1 1 1] 적을 만들고 싶다
    (`|SpawnActorFromClass` "/Game/Shooting/BP_Enemy.BP_Enemy_C" (`KismetMathLibrary.MakeTransform` (`self.K2_GetActorLocation`)) "Undefined" "MultiplyWithRoot" null null)
    (set `self.CurrentTime` 0.0)))

(fn `TimeFlow`
  (params (A :type "Float (double-precision)"))
  (set `self.CurrentTime` (+ A (`self.CurrentTime`))))

(fn `UserConstructionScript`)